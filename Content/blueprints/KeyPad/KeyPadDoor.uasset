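; KeyPadDoor is a sliding classroom door with a lock flag, driven by a Box trigger and a test input action.
; Pressing Test calls OpenDoor when unlocked, playing the DoorOpening timeline to move the mesh along relative X.
; The player leaving the Box calls CloseDoor, which reverses the timeline.
; EnableDoor, called on player entry, and LockDoor, called when locked, are empty stubs, so Test is not gated by proximity here.
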(event `self.Box.OnComponentBeginOverlap`
  (params (OverlappedComponent :type "PrimitiveComponent Object Reference") (OtherActor :type "Actor Object Reference") (OtherComp :type "PrimitiveComponent Object Reference") (OtherBodyIndex :type Integer) (bFromSweep :type Boolean) (SweepResult :type "HitResult Structure (by ref)"))
  ;[1 1 1] 코멘트
  (if (== OtherActor (`GameplayStatics.GetPlayerCharacter` 0))
    (`self.EnableDoor`)))

(event `InputAction|Test`
  (params (Key :type "Key Structure"))
  (:`Pressed`
    (if (`self.IsLocked`)
      (`self.LockDoor`)
      (else
        (`self.OpenDoor`)))))

(event `self.Box.OnComponentEndOverlap`
  (params (OverlappedComponent :type "PrimitiveComponent Object Reference") (OtherActor :type "Actor Object Reference") (OtherComp :type "PrimitiveComponent Object Reference") (OtherBodyIndex :type Integer))
  ;[1 1 1] 코멘트
  (if (== (`GameplayStatics.GetPlayerCharacter` 0) OtherActor)
    (`self.CloseDoor`)))

(event `OpenDoor`
  (set `self.IsOpen` true)
  (`KismetSystemLibrary.PrintString` "문이열렸다")
  (bind (_direction _dooropening) (`Timeline|DoorOpening` :!label _label)
    (:`Update`
      (`SceneComponent.K2_SetRelativeLocation` (`self.교실_벽_앞문`) (`KismetMathLibrary.MakeVector` _dooropening) false false))))

(event `CloseDoor`
  (set `self.IsOpen` false)
  (`KismetSystemLibrary.PrintString` "문이닫혔다")
  (goto _label :!via `Reverse`))

(event `LockDoor`)

(event `EnableDoor`)

(fn `UserConstructionScript`)