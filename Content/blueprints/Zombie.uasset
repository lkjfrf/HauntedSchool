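; Zombie enemy character that walks at a set ground speed and melee-attacks any Student entering its Box trigger.
; An overlap plays the attack montage, applies light damage immediately and halts movement for a few seconds.
; A DoOnce gate blocks repeat hits until the delay restores walk speed and calls ResetAttack.
; MeleeAttack and DamagePlayer are empty events.
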(event `/Game/Animation/zombie/CombatInterface.MeleeAttack`)

(event `DamagePlayer`)

(event `self.ReceiveBeginPlay`
  (set `CharacterMovementComponent.MaxWalkSpeed` (`self.WalkGroundSpeed`) (`self.CharacterMovement`)))

(event `self.Box.OnComponentBeginOverlap`
  (params (OverlappedComponent :type "PrimitiveComponent Object Reference") (OtherActor :type "Actor Object Reference") (OtherComp :type "PrimitiveComponent Object Reference") (OtherBodyIndex :type Integer) (bFromSweep :type Boolean) (SweepResult :type "HitResult Structure (by ref)"))
  (bind _charactermovement (`self.CharacterMovement`))
  (bind _asstudent (cast `/Game/blueprints/Student` OtherActor))
  (`/Engine/EditorBlueprintResources/StandardMacros.DoOnce` false :!label _label
    (:`Completed`
      (`AnimInstance.Montage_Play` (`SkeletalMeshComponent.GetAnimInstance` (`self.Mesh`)) "/Game/Animation/zombie/zombieattack_Anim_Montage.zombieattack_Anim_Montage" 1.0 "MontageLength" 0.0 true)
      (`GameplayStatics.ApplyDamage` _asstudent 0.3 (`self.GetController` self))
      (set `CharacterMovementComponent.MaxWalkSpeed` 0.0 _charactermovement)
      (`KismetSystemLibrary.Delay` 4.0)
      (set `CharacterMovementComponent.MaxWalkSpeed` (`self.WalkGroundSpeed`) _charactermovement)
      (`self.ResetAttack`))))

(event `ResetAttack`
  (goto _label :!via `Reset`))

(fn `UserConstructionScript`)