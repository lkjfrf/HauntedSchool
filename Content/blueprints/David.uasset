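; David is a character Blueprint for what appears to be a chasing dorm supervisor that damages what it catches, with walk and sprint speeds.
; BeginSprint and EndSprint switch max walk speed and the IsSprint flag, starting at walk speed.
; A Reset-linked DoOnce chain plays an attack montage, waits, damages the overlapped actor, then calls Reset.
; The Box overlap and MeleeAttack_david events have no execution wired.
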(event `MeleeAttack_david`)

(event `self.ReceiveBeginPlay`
  (set `CharacterMovementComponent.MaxWalkSpeed` (`self.WalkGroundSpeed`) (`self.CharacterMovement`)))

(event `self.Box.OnComponentBeginOverlap`
  (params (OverlappedComponent :type "PrimitiveComponent Object Reference") (OtherActor :type "Actor Object Reference") (OtherComp :type "PrimitiveComponent Object Reference") (OtherBodyIndex :type Integer) (bFromSweep :type Boolean) (SweepResult :type "HitResult Structure (by ref)"))
  ;[1 1 1] 사감에게 쫒겨서 닿을시 데미지
)

(event `Reset`
  ;[1 1 1] 사감에게 쫒겨서 닿을시 데미지
  (`/Engine/EditorBlueprintResources/StandardMacros.DoOnce` false :!via `Reset`
    (:`Completed`
      (`AnimInstance.Montage_Play` (`SkeletalMeshComponent.GetAnimInstance` (`self.Mesh`)) "/Game/Animation/david/davidattack_Anim_Montage.davidattack_Anim_Montage" 1.0 "MontageLength" 0.0 true)
      (`KismetSystemLibrary.Delay` 0.9)
      (`GameplayStatics.ApplyDamage` (stale `self.Box.OnComponentBeginOverlap` OtherActor) 100.0)
      (`self.Reset`))))

(fn `BeginSprint`
  ;[1 1 1] 스프린트를 시작하면 스프린트 그라운드 스피드로 전환
  (set `CharacterMovementComponent.MaxWalkSpeed` (`self.SprintGroundSpeed`) (`self.CharacterMovement`))
  (set `self.IsSprint` true))

(fn `EndSprint`
  ;[1 1 1] 스프린트를 멈추면 다시 걷기속도로
  (set `CharacterMovementComponent.MaxWalkSpeed` (`self.WalkGroundSpeed`) (`self.CharacterMovement`))
  (set `self.IsSprint` false))

(fn `UserConstructionScript`)