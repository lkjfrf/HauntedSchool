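; Light_BP_2 is a light Blueprint that makes its point light pulse irregularly between a minimum and maximum intensity.
; Each Tick moves the intensity toward a target at the constant PulseRate using FInterpToConstant.
; When the intensity equals the target, a new random target is picked within MinIntensity and MaxIntensity.
; BeginPlay and the construction script contain no logic.
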(event `self.ReceiveTick`
  (params (DeltaSeconds :type "Float (single-precision)"))
  (if (== (`LightComponentBase.Intensity` (`self.PointLightComponent`)) (`self.Target_Intensity`))
    (set `self.Target_Intensity` (`KismetMathLibrary.RandomFloatInRange` (`self.Min_Intensity`) (`self.Max_Intensity`)))
    (else
      (`LightComponent.SetIntensity` (`self.PointLightComponent`) (`KismetMathLibrary.FInterpTo_Constant` (`LightComponentBase.Intensity` (`self.PointLightComponent`)) (`self.Target_Intensity`) DeltaSeconds (`self.Pulse_Rate`))))))

(fn `UserConstructionScript`)