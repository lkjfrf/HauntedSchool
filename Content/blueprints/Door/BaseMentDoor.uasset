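; Basement door Blueprint that swings its static mesh open and closed around yaw through a timeline.
; ToggleDoor plays or reverses the timeline depending on the current RotateZ value.
; Timeline updates drive the rotation and feed a 60-second Delay that then reverses the timeline, closing the door automatically.
; A box trigger records Student overlap in BoxOverlap, which only an unreachable branch reads.
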(event `ToggleDoor`
  (if (< (stale _rotatez) 1.0)
    (bind (_direction _rotatez) (`Timeline|타임라인_0` :!label _label)
      (:`Update`
        (`SceneComponent.K2_SetRelativeRotation` (`self.StaticMesh`) (`KismetMathLibrary.MakeRotator` 0.0 0.0 _rotatez) false false)
        (`KismetSystemLibrary.Delay` 60.0)
        (goto _label :!via `Reverse`)))
    (else
      (goto _label :!via `Reverse`))))

(event `self.Box.OnComponentBeginOverlap`
  (params (OverlappedComponent :type "PrimitiveComponent Object Reference") (OtherActor :type "Actor Object Reference") (OtherComp :type "PrimitiveComponent Object Reference") (OtherBodyIndex :type Integer) (bFromSweep :type Boolean) (SweepResult :type "HitResult Structure (by ref)"))
  (cast `/Game/blueprints/Student` OtherActor)
  (set `self.BoxOverlap?` true))

(event `self.Box.OnComponentEndOverlap`
  (params (OverlappedComponent :type "PrimitiveComponent Object Reference") (OtherActor :type "Actor Object Reference") (OtherComp :type "PrimitiveComponent Object Reference") (OtherBodyIndex :type Integer))
  (cast `/Game/blueprints/Student` OtherActor)
  (set `self.BoxOverlap?` false))

(fn `UserConstructionScript`)