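; MasterItem is a pickup item actor that highlights and shows an icon when a Student is nearby.
; BeginPlay links the widget component's WB_ItemIcon to the item, applies the mesh from Details, and creates a separate WB_ItemIcon stored in ItemIcon0.
; Overlap begin and end toggle the widget and custom-depth focus highlight.
; Both events set the Student's PickableItem to this item, so leaving does not clear it.
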(event `self.ReceiveBeginPlay`
  (bind _aswb_item_icon (cast `/Game/UI/GamePlay/WB_ItemIcon` (`WidgetComponent.GetUserWidgetObject` (`self.Widget`))))
  (bind _output_get (set `/Game/UI/GamePlay/WB_ItemIcon.OwningItem` self _aswb_item_icon))
  (`StaticMeshComponent.SetStaticMesh` (`self.ItemMesh`) (`.ItemMesh_23_1B190C32491D881F27A43195A8D8ACAC` (break `/Game/blueprints/Item/S_ItemDetails` (`/Game/blueprints/Item/MasterItem.Details` _output_get))))
  (bind _returnvalue (`|CreateWidget` "/Game/UI/GamePlay/WB_ItemIcon.WB_ItemIcon_C"))
  (set `self.ItemIcon_0` _returnvalue))

(event `self.OverlapCollision.OnComponentBeginOverlap`
  (params (OverlappedComponent :type "PrimitiveComponent Object Reference") (OtherActor :type "Actor Object Reference") (OtherComp :type "PrimitiveComponent Object Reference") (OtherBodyIndex :type Integer) (bFromSweep :type Boolean) (SweepResult :type "HitResult Structure (by ref)"))
  (bind _asstudent (cast `/Game/blueprints/Student` OtherActor))
  (set `/Game/blueprints/Student.PickableItem` self _asstudent)
  (`PrimitiveComponent.SetRenderCustomDepth` (`self.ItemMesh`) false)
  (`self.BeginFocus`)
  (`SceneComponent.SetVisibility` (`self.Widget`) true false))

(event `self.OverlapCollision.OnComponentEndOverlap`
  (params (OverlappedComponent :type "PrimitiveComponent Object Reference") (OtherActor :type "Actor Object Reference") (OtherComp :type "PrimitiveComponent Object Reference") (OtherBodyIndex :type Integer))
  (bind _asstudent (cast `/Game/blueprints/Student` OtherActor))
  (set `/Game/blueprints/Student.PickableItem` self _asstudent)
  (`self.EndFocus`)
  (`SceneComponent.SetVisibility` (`self.Widget`) false false))

(fn `BeginFocus`
  (`PrimitiveComponent.SetRenderCustomDepth` (`self.ItemMesh`) true))

(fn `EndFocus`
  (`PrimitiveComponent.SetRenderCustomDepth` (`self.ItemMesh`) false))

(fn `UserConstructionScript`)