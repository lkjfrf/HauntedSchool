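; Doll enemy character that attacks the Student player and reports its proximity.
; Overlapping its Box deals slight damage and sets the anim Blueprint's Attacking flag for four seconds.
; Tick sets the player controller's DollInrange flag by distance.
; A DoOnce attack sequence with camera blend, input lock and heavy damage call has its entry disconnected, so it never plays.
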(event `self.ReceiveBeginPlay`
  (set `CharacterMovementComponent.MaxWalkSpeed` (`self.WalkGroundSpeed`) (`self.CharacterMovement`)))

(event `Reset`
  (bind _returnvalue (`GameplayStatics.GetPlayerController` 0))
  (bind _returnvalue_2 (`GameplayStatics.GetPlayerController` 0))
  (bind _aspnanim_bp_doll (cast `/Game/Animation/PNAnimBP_doll` (`SkeletalMeshComponent.GetAnimInstance` (`self.Mesh`)) :!pure true))
  ;[1 1 1] 공격시 데미지
  (`/Engine/EditorBlueprintResources/StandardMacros.DoOnce` false :!via `Reset`
    (:`Completed`
      (`PlayerController.SetViewTargetWithBlend` (`GameplayStatics.GetPlayerController` 0) self 0.0 "VTBlend_Linear" 1.0 false)
      (`Controller.SetIgnoreMoveInput` _returnvalue_2 true)
      (`Controller.SetIgnoreLookInput` _returnvalue_2 true)
      (set `/Game/Animation/PNAnimBP_doll.Attacking` true _aspnanim_bp_doll)
      (`KismetSystemLibrary.Delay` 4.0)
      (set `/Game/Animation/PNAnimBP_doll.Attacking` false _aspnanim_bp_doll)
      (`GameplayStatics.ApplyDamage` null 100.0)
      (`PlayerController.SetViewTargetWithBlend` _returnvalue (`GameplayStatics.GetPlayerCharacter` 0) 3.0 "VTBlend_Linear" 0.0 false)
      (`Controller.ResetIgnoreLookInput` _returnvalue)
      (`Controller.ResetIgnoreMoveInput` _returnvalue)
      (`self.Reset`)
      (set `CharacterMovementComponent.MaxWalkSpeed` 600.0 (`self.CharacterMovement`)))))

(event `self.Box.OnComponentBeginOverlap`
  (params (OverlappedComponent :type "PrimitiveComponent Object Reference") (OtherActor :type "Actor Object Reference") (OtherComp :type "PrimitiveComponent Object Reference") (OtherBodyIndex :type Integer) (bFromSweep :type Boolean) (SweepResult :type "HitResult Structure (by ref)"))
  (bind _aspnanim_bp_doll (cast `/Game/Animation/PNAnimBP_doll` (`SkeletalMeshComponent.GetAnimInstance` (`self.Mesh`)) :!pure true))
  (cast `/Game/blueprints/Student` OtherActor)
  (`GameplayStatics.ApplyDamage` OtherActor 0.3 (`self.GetController` self))
  (set `/Game/Animation/PNAnimBP_doll.Attacking` true _aspnanim_bp_doll)
  (`KismetSystemLibrary.Delay` 4.0)
  (set `/Game/Animation/PNAnimBP_doll.Attacking` false _aspnanim_bp_doll))

(event `self.ReceiveTick`
  (params (DeltaSeconds :type "Float (single-precision)"))
  (bind _asstudent (cast `/Game/blueprints/Student` (`GameplayStatics.GetPlayerCharacter` 0) :!pure true))
  (bind _asgame_play_pc (cast `/Game/blueprints/GamePlay/GamePlayPC` (`self.GetController` _asstudent) :!pure true))
  (if (<= (`self.GetDistanceTo` self _asstudent) 900.0)
    (set `/Game/blueprints/GamePlay/GamePlayPC.Doll_Inrange` true _asgame_play_pc)
    (else
      (set `/Game/blueprints/GamePlay/GamePlayPC.Doll_Inrange` false _asgame_play_pc))))

(fn `UserConstructionScript`)