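; NPC Blueprint that shows data-table-driven dialogue, advancing one line each time it is interacted with.
; BeginPlay caches DialogueExcel rows matching its NPCID; Interact increments LineID and picks text by ConversationID and LineID.
; A DialogueItem widget displays the line and resets when no single match exists, while leaving the box removes it from view.
; The construction script passes DialogueTree to the NPC_AI controller.
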(event `self.ReceiveBeginPlay`
  (bind _outrownames (`DataTableFunctionLibrary.GetDataTableRowNames` "/Game/Test/DialogueExcel.DialogueExcel"))
  (for _array_element _outrownames
    (bind _returnvalue (`|GetDataTableRow` "/Game/Test/DialogueExcel.DialogueExcel" _array_element)
      (:`then`
        (if (== (`.NPC_ID_8_34FB46A6492203C7160587BEF010FE01` (break `/Game/Test/DialogueStructure` _returnvalue)) (`self.NPC_ID`))
          (`KismetArrayLibrary.Array_Add` (`self.Dialogue`) _array_element))))))

(event `/Game/Test/InteractDialogue.Interact`
  (`/Engine/EditorBlueprintResources/StandardMacros.IncrementInt` (`self.Line_ID`)
    (:`  `
      (`self.DialogueCreate`))))

(event `self.Box.OnComponentBeginOverlap`
  (params (OverlappedComponent :type "PrimitiveComponent Object Reference") (OtherActor :type "Actor Object Reference") (OtherComp :type "PrimitiveComponent Object Reference") (OtherBodyIndex :type Integer) (bFromSweep :type Boolean) (SweepResult :type "HitResult Structure (by ref)")))

(event `self.Box.OnComponentEndOverlap`
  (params (OverlappedComponent :type "PrimitiveComponent Object Reference") (OtherActor :type "Actor Object Reference") (OtherComp :type "PrimitiveComponent Object Reference") (OtherBodyIndex :type Integer))
  (bind _dialogue_rf (`self.Dialogue RF`))
  (`/Engine/EditorBlueprintResources/StandardMacros.IsValid` _dialogue_rf
    (:`Is Valid`
      (`Widget.RemoveFromParent` _dialogue_rf))))

(fn `DialogueCreate`
  (`/Engine/EditorBlueprintResources/StandardMacros.IsValid` (`self.Dialogue RF`)
    (:`Is Valid`
      (bind _line (`self.DialogueGetLine`))
      (set `/Game/Test/DialogueItem.DialogueText` _line (`self.Dialogue RF`)))
    (:`Is Not Valid`
      (bind _returnvalue (`|CreateWidget` "/Game/Test/DialogueItem.DialogueItem_C" (`GameplayStatics.GetPlayerController` 0)))
      (bind _output_get (set `self.Dialogue RF` _returnvalue))
      (`UserWidget.AddToViewport` _output_get 0)
      (bind _line_2 (`self.DialogueGetLine`))
      (set `/Game/Test/DialogueItem.DialogueText` _line_2 (`self.Dialogue RF`)))))

(fn `DialogueGetLine`
  (returns (Line :type Text))
  (locals (ReturnLine :type "Array of Text"))
  (for _array_element (`self.Dialogue`)
    (bind _returnvalue (`|GetDataTableRow` "/Game/Test/DialogueExcel.DialogueExcel" _array_element) ; 현재행이랑 맞는 대사행 가져오기
      (:`then`
        (bind (_npc_id _conversation_id _line_id _dialogue) (break `/Game/Test/DialogueStructure` _returnvalue))
        (if (and (== _conversation_id (`self.Conversation_ID`)) (== _line_id (`self.Line_ID`)))
          (`KismetArrayLibrary.Array_Add` (`local.ReturnLine`) _dialogue)))))
  (if (== (`KismetArrayLibrary.Array_Length` (`local.ReturnLine`)) 1)
    (return (`|GetArrayItem` (`local.ReturnLine`)))
    (else
      (`Widget.RemoveFromParent` (`self.Dialogue RF`))
      (set `self.Dialogue RF` null) ; 초기화
      (set `self.Line_ID` 0))))

(fn `UserConstructionScript`
  (bind _asnpc_ai (cast `/Game/AI/NPC/NPC_AI` (`AIBlueprintHelperLibrary.GetAIController` self)))
  (set `/Game/AI/NPC/NPC_AI.DialogueTree` (`self.DialogueTree`) _asnpc_ai))