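; Guard character, a dorm supervisor that chases and attacks Student characters, with functions to switch between walk and sprint speed.
; A Box overlap with a Student plays the attack montage, applies damage and halts the Guard briefly, using a DoOnce as cooldown.
; A camera-takeover kill sequence with locked player input hangs off a second DoOnce whose Enter is never triggered, leaving it inactive.
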(event `self.ReceiveBeginPlay`
  (set `CharacterMovementComponent.MaxWalkSpeed` (`self.WalkGroundSpeed`) (`self.CharacterMovement`)))

(event `Reset`
  (bind _returnvalue (`GameplayStatics.GetPlayerController` 0))
  (bind _returnvalue_2 (`GameplayStatics.GetPlayerController` 0))
  ;[1 1 1] 사감에게 쫒겨서 닿을시 데미지
  (`/Engine/EditorBlueprintResources/StandardMacros.DoOnce` false :!via `Reset`
    (:`Completed`
      (`PlayerController.SetViewTargetWithBlend` (`GameplayStatics.GetPlayerController` 0) self 0.0 "VTBlend_Linear" 1.0 false)
      (`Controller.SetIgnoreMoveInput` _returnvalue_2 true)
      (`Controller.SetIgnoreLookInput` _returnvalue_2 true)
      (`AnimInstance.Montage_Play` (`SkeletalMeshComponent.GetAnimInstance` (`self.Mesh`)) "/Game/Animation/david/davidattack_Anim_Montage.davidattack_Anim_Montage" 1.0 "MontageLength" 0.0 true)
      (`KismetSystemLibrary.Delay` 1.0)
      (`GameplayStatics.ApplyDamage` null 100.0)
      (`KismetSystemLibrary.Delay` 3.0)
      (`PlayerController.SetViewTargetWithBlend` _returnvalue (`GameplayStatics.GetPlayerCharacter` 0) 3.0 "VTBlend_Linear" 0.0 false)
      (`Controller.ResetIgnoreLookInput` _returnvalue)
      (`Controller.ResetIgnoreMoveInput` _returnvalue)
      (`self.Reset`))))

(event `self.Box.OnComponentBeginOverlap`
  (params (OverlappedComponent :type "PrimitiveComponent Object Reference") (OtherActor :type "Actor Object Reference") (OtherComp :type "PrimitiveComponent Object Reference") (OtherBodyIndex :type Integer) (bFromSweep :type Boolean) (SweepResult :type "HitResult Structure (by ref)"))
  (bind _charactermovement (`self.CharacterMovement`))
  (bind _asstudent (cast `/Game/blueprints/Student` OtherActor))
  (`/Engine/EditorBlueprintResources/StandardMacros.DoOnce` false :!label _label
    (:`Completed`
      (`AnimInstance.Montage_Play` (`SkeletalMeshComponent.GetAnimInstance` (`self.Mesh`)) "/Game/Animation/david/davidattack_Anim_Montage.davidattack_Anim_Montage" 1.0 "MontageLength" 0.0 true)
      (`GameplayStatics.ApplyDamage` _asstudent 0.25 (`self.GetController` self))
      (set `CharacterMovementComponent.MaxWalkSpeed` 0.0 _charactermovement)
      (`KismetSystemLibrary.Delay` 4.0)
      (set `CharacterMovementComponent.MaxWalkSpeed` (`self.WalkGroundSpeed`) _charactermovement)
      (`self.ResetAttack`))))

(event `ResetAttack`
  (goto _label :!via `Reset`))

(fn `BeginSprint`
  (set `CharacterMovementComponent.MaxWalkSpeed` (`self.SprintGroundSpeed`) (`self.CharacterMovement`))
  (set `self.IsSprint?` true))

(fn `EndSprint`
  (set `CharacterMovementComponent.MaxWalkSpeed` (`self.WalkGroundSpeed`) (`self.CharacterMovement`))
  (set `self.IsSprint?` false))

(fn `UserConstructionScript`)