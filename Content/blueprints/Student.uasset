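; Networked student player character with first/third-person cameras, stamina-limited sprinting, an inventory, dialogue and line-trace door interaction, some doors needing held keys.
; Client/server event pairs sync movement, pickups, drops and equipping, while look rotation is multicast to drive remote spring arms.
; A RepNotify slot attaches the held item mesh and sets the matching animation blendspace.
; Damage blends the view to the attacker, teleports the student, then restores control.
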(event `self.ReceiveBeginPlay`
  (set `self.Student1?` (== (`SkeletalMeshComponent.AnimClass` (`self.Mesh`)) "/Game/Animation/PNAnimBP_Student.PNAnimBP_Student_C")))

(event `self.ReceiveTick`
  (params (DeltaSeconds :type "Float (single-precision)"))
  (bind _1personspringarm (`self.1PersonSpringArm`))
  (bind _3personspringarm (`self.3PersonSpringArm`))
  ;[1 1 1] Tick
  (`|ExecutionSequence`
    (:`then_2`
      ;;[1 1 1] FirstPersonCamera 스프링암 멀티케스트
      (`/Engine/EditorBlueprintResources/ActorMacros.Switch Has Authority`
        (:`Authority`
          (if (`KismetSystemLibrary.IsServer`)
            (`self.SetLookRotation_Multicast` (`self.GetControlRotation`))))
        (:`Remote`
          (if (!= (`GameplayStatics.GetPlayerPawn` 0) self)
            (set `SpringArmComponent.bUsePawnControlRotation` false _3personspringarm) ; Look Rotation으로 회전하기 위해 disable
            (set `SpringArmComponent.bUsePawnControlRotation` false _1personspringarm) ; Look Rotation으로 회전하기 위해 disable
            (else
              (set `SpringArmComponent.bUsePawnControlRotation` true _3personspringarm)
              (set `SpringArmComponent.bUsePawnControlRotation` true _1personspringarm)))
          (`SceneComponent.K2_SetWorldRotation` _1personspringarm (`self.LookRotation`) false false)
          (`SceneComponent.K2_SetWorldRotation` _3personspringarm (`self.LookRotation`) false false))))))

(event `SetLookRotation_Multicast`
  (params (LookRotation :type "Rotator Structure"))
  ;[1 1 1] Tick
  ;;[1 1 1] FirstPersonCamera 스프링암 멀티케스트
  (if (!= (`GameplayStatics.GetPlayerPawn` 0) self)
    (set `self.LookRotation` LookRotation)))

(event `Jumping_Client`
  (params (IsJumping :type Boolean))
  ;[1 1 1] 점프
  (`self.Jumping_Server` IsJumping))

(event `Jumping_Server`
  (params (IsJumping :type Boolean))
  ;[1 1 1] 점프
  (set `self.IsJumping` IsJumping))

(event `InputAction|InteractItem`
  (params (Key :type "Key Structure"))
  ;[1 1 1] 다디얼로그
  (:`Pressed`
    (`|ExecutionSequence`
      (:`then_0`
        (`self.PickItem_Client`))
      (:`then_1`
        (bind _outactors (`GameplayStatics.GetAllActorsWithInterface` "/Game/Test/InteractDialogue.InteractDialogue_C"))
        (for _array_element _outactors
          (if (`self.IsOverlappingActor` _array_element self)
            (message `/Game/Test/InteractDialogue.Interact` _array_element)))))))

(event `DecreaseStamina`
  ;[1 1 1] 달리기
  (bind _output_get (set `self.CurrentStamina` (`KismetMathLibrary.FClamp` (- (`self.CurrentStamina`) (`self.DecreaseStaminaRate`)) 0.0 (`self.MaxStamina`))))
  ;;[1 1 1] 스테미나 떨어질시 못달리게
  (if (== _output_get 0.0)
    (`self.StopSprint_Client` 300.0 (stale `StartSprint_Client` `타깃`))))

(event `StartSprint_Client`
  (params (MaxWalkSpeed :type "Float (double-precision)") (`타깃` :type "CharacterMovementComponent Object Reference"))
  ;[1 1 1] 달리기
  (`self.StartSprint_Server` MaxWalkSpeed `타깃`)
  (set `CharacterMovementComponent.MaxWalkSpeed` MaxWalkSpeed (`self.CharacterMovement`))
  (`KismetSystemLibrary.K2_ClearAndInvalidateTimerHandle` (`self.IncreaseStaminaHandle`)) ; 이걸 설정안하면 증가와 감소 같은 시간에 발동됨
  (bind _returnvalue (`KismetSystemLibrary.K2_SetTimerDelegate` (delegate `DecreaseStamina`) 0.1 true)) ; 서버오버로드 줄이기
  (set `self.DecreaseStaminaHandle` _returnvalue))

(event `PickItem_Client`
  (bind _pickableitem (`self.PickableItem`))
  ;[1 1 1] 아이템 줍기
  (`/Engine/EditorBlueprintResources/StandardMacros.IsValid` _pickableitem
    (:`Is Valid`
      (`KismetArrayLibrary.Array_Add` (`self.Inventory`) (`/Game/blueprints/Item/MasterItem.Details` _pickableitem)) ; 소유 클라이언트에서 인벤토리에 추가하고 엑터삭제는 서버, 클라이언트 둘다 동시에 삭제
      (`self.DestroyItem_Server` _pickableitem))))

(event `CustomEvent_1`
  (bind _asgame_play_pc (cast `/Game/blueprints/GamePlay/GamePlayPC` (`self.GetController`) :!pure true))
  ;[1 1 1] 스크립트 출력
  (`/Engine/EditorBlueprintResources/StandardMacros.DoOnce` false :!via `Reset`
    (:`Completed`
      (bind _returnvalue (`|CreateWidget` "/Game/UI/GamePlay/Script.Script_C" _asgame_play_pc))
      (`UserWidget.AddToViewport` _returnvalue 0)
      (`WidgetBlueprintLibrary.SetInputMode_GameAndUIEx` _asgame_play_pc null "LockAlways")
      (bind _output_get (set `/Game/UI/GamePlay/Script.ScriptLines` _ _returnvalue))
      (set `/Game/UI/GamePlay/Script.NumOfLine` (`KismetArrayLibrary.Array_Length` _output_get) _returnvalue))))

(event `StartSprint_Server`
  (params (MaxWalkSpeed :type "Float (double-precision)") (CharMovementComponent :type "CharacterMovementComponent Object Reference"))
  ;[1 1 1] 달리기
  (set `CharacterMovementComponent.MaxWalkSpeed` MaxWalkSpeed CharMovementComponent)
  (set `self.IsSprinting` true))

(event `IncreaseStamina`
  ;[1 1 1] 달리기
  (set `self.CurrentStamina` (`KismetMathLibrary.FClamp` (+ (`self.CurrentStamina`) (`self.IncreaseStaminaRate`)) 0.0 (`self.MaxStamina`))))

(event `StopSprint_Client`
  (params (MaxWalkSpeed :type "Float (double-precision)") (`타깃` :type "CharacterMovementComponent Object Reference"))
  ;[1 1 1] 달리기
  (`self.StopSprint_Server` MaxWalkSpeed `타깃`)
  (set `CharacterMovementComponent.MaxWalkSpeed` MaxWalkSpeed (`self.CharacterMovement`))
  (`KismetSystemLibrary.K2_ClearAndInvalidateTimerHandle` (`self.DecreaseStaminaHandle`))
  (bind _returnvalue (`KismetSystemLibrary.K2_SetTimerDelegate` (delegate `IncreaseStamina`) 0.1 true)) ; 서버오버로드 줄이기
  (set `self.IncreaseStaminaHandle` _returnvalue))

(event `DestroyItem_Server`
  (params (`타깃` :type "Actor Object Reference"))
  ;[1 1 1] 아이템 줍기
  (`self.K2_DestroyActor` `타깃`) ; 서버에서는 엑터삭제만 해야함 (인벤토리 추가 X)
)

(event `StopSprint_Server`
  (params (MaxWalkSpeed :type "Float (double-precision)") (`타깃` :type "CharacterMovementComponent Object Reference"))
  ;[1 1 1] 달리기
  (set `CharacterMovementComponent.MaxWalkSpeed` MaxWalkSpeed `타깃`)
  (set `self.IsSprinting` false))

(event `PrintScript`
  (params (ScriptLines :type "Array of Text") (`DoOnce?` :type Boolean))
  ;[1 1 1] 스크립트 출력
  (bind _returnvalue (`|CreateWidget` "/Game/UI/GamePlay/Script.Script_C" (cast `/Game/blueprints/GamePlay/GamePlayPC` (`self.GetController`) :!pure true)))
  (`UserWidget.AddToViewport` _returnvalue 0)
  (bind _output_get (set `/Game/UI/GamePlay/Script.ScriptLines` ScriptLines _returnvalue))
  (set `/Game/UI/GamePlay/Script.NumOfLine` (`KismetArrayLibrary.Array_Length` _output_get) _returnvalue))

(event `InputAction|InteractLookAt`
  (params (Key :type "Key Structure"))
  ;[1 1 1] E버튼 아이템상호작용
  (:`Pressed`
    (`/Engine/EditorBlueprintResources/ActorMacros.Switch Has Authority`
      (:`Authority`
        (`self.Look_Client`)
        (`self.InteractMulti`))
      (:`Remote`
        (`self.Look_Server`)
        (`self.InteractServer`)))))

(event `SetAimRot_Client`
  (params (AimRotation :type "Rotator Structure"))
  ;[1 1 1] 에임 로테이션 설정 (머리방향)
  (`self.SetAimRot_Server` AimRotation))

(event `Key|V`
  (params (Key :type "Key Structure"))
  ;[1 1 1] 1인칭 3인칭 변경
  (:`Pressed`
    (`/Engine/EditorBlueprintResources/StandardMacros.FlipFlop`
      (:`A`
        (`ActorComponent.Deactivate` (`self.ADSCamera`))
        (`ActorComponent.Activate` (`self.FirstPersonCamera`) false)
        (set `self.FirstPersonCamera?` true))
      (:`B`
        (`ActorComponent.Deactivate` (`self.FirstPersonCamera`))
        (`ActorComponent.Activate` (`self.ADSCamera`) false)
        (set `self.FirstPersonCamera?` false)))))

(event `InteractServer`
  ;[1 1 1] E버튼 아이템상호작용
  (`self.InteractMulti`))

(event `InteractMulti`
  ;[1 1 1] E버튼 아이템상호작용
  (bind _lookatactor (`self.LookAtActor`)
    (:`then`
      (`|ExecutionSequence`
        (:`then_0`
          (bind _asred_locker_door (cast `/Game/blueprints/Door/RedLockerDoor` _lookatactor))
          (`/Game/blueprints/Door/RedLockerDoor.ToggleLockerDoor` _asred_locker_door))
        (:`then_1`
          (bind _asdoor (cast `/Game/blueprints/Door/Door` _lookatactor))
          (`/Game/blueprints/Door/Door.ToggleDoor` _asdoor))
        (:`then_2`
          (bind _asart_door (cast `/Game/blueprints/Door/ArtDoor` _lookatactor))
          ;[1 1 1] 열쇠를 들고있어야만 문열림
          (if (== (`StaticMeshComponent.StaticMesh` (`self.UseItemMesh`)) "/Game/Maps/NormalClass/Items_Key.Items_Key")
            (`/Game/blueprints/Door/ArtDoor.ToggleDoor` _asart_door)))
        (:`then_3`
          (bind _asbath_room_door (cast `/Game/blueprints/Door/BathRoomDoor` _lookatactor))
          (`/Game/blueprints/Door/BathRoomDoor.ToggleDoor` _asbath_room_door))
        (:`then_4`
          (bind _asclass_door (cast `/Game/blueprints/Door/ClassDoor` _lookatactor))
          (`/Game/blueprints/Door/ClassDoor.ToggleDoor` _asclass_door))
        (:`then_5`
          (bind _asgreen_locker_door (cast `/Game/blueprints/Door/GreenLockerDoor` _lookatactor))
          (`/Game/blueprints/Door/GreenLockerDoor.ToggleLockerDoor` _asgreen_locker_door))
        (:`then_6`
          (bind _asbase_ment_door (cast `/Game/blueprints/Door/BaseMentDoor` _lookatactor))
          (`/Game/blueprints/Door/BaseMentDoor.ToggleDoor` _asbase_ment_door))
        (:`then_7`
          (bind _asmain_door (cast `/Game/blueprints/Door/MainDoor` _lookatactor))
          ;[1 1 1] 파란열쇠 + 사진있어야 열림
          (if (== (`StaticMeshComponent.StaticMesh` (`self.UseItemMesh`)) "/Game/Maps/NormalClass/Items_Key2.Items_Key2")
            (`/Game/blueprints/Door/MainDoor.MainDoorOpen` _asmain_door)))))
    (:`else`)))

(event `SetAimRot_Server`
  (params (AimRotation :type "Rotator Structure"))
  ;[1 1 1] 에임 로테이션 설정 (머리방향)
  (set `self.AimRotation` AimRotation))

(event `self.ReceiveAnyDamage`
  (params (Damage :type "Float (single-precision)") (DamageType :type "DamageType Object Reference") (InstigatedBy :type "Controller Object Reference") (DamageCauser :type "Actor Object Reference"))
  (bind _asgame_play_pc (cast `/Game/blueprints/GamePlay/GamePlayPC` (`self.GetController`) :!pure true))
  ;[1 1 1] 데미지 입었을때
  (`/Game/blueprints/GamePlay/GamePlayPC.TakeDamage` (cast `/Game/blueprints/GamePlay/GamePlayPC` (`self.GetController`) :!pure true) Damage)
  (`/Engine/EditorBlueprintResources/StandardMacros.DoOnce` false :!label _label
    (:`Completed`
      (`PlayerController.SetViewTargetWithBlend` _asgame_play_pc (`Controller.K2_GetPawn` InstigatedBy) 0.0 "VTBlend_Linear" 1.0 false) ; 공격당한대상과 카메라합치기
      (`Controller.SetIgnoreMoveInput` _asgame_play_pc true)
      (`Controller.SetIgnoreLookInput` _asgame_play_pc true)
      (`KismetSystemLibrary.Delay` 1.0)
      (`self.K2_SetActorLocation` (2670.0 -1795.0 -50.0) false true)
      (`KismetSystemLibrary.Delay` 3.0)
      (`PlayerController.SetViewTargetWithBlend` _asgame_play_pc self 3.0 "VTBlend_Linear" 0.0 false)
      (`Controller.ResetIgnoreLookInput` _asgame_play_pc)
      (`Controller.ResetIgnoreMoveInput` _asgame_play_pc)
      (`self.Reset`))))

(event `Reset`
  ;[1 1 1] 데미지 입었을때
  (goto _label :!via `Reset`))

(event `Look_Server`
  ;[1 1 1] 보고있는것 라인트레이스로 확인하기
  (`self.Look_Client`))

(event `Look_Client`
  (bind _firstpersoncamera (`self.FirstPersonCamera`))
  (bind _adscamera (`self.ADSCamera`))
  (bind _returnvalue (`SceneComponent.K2_GetComponentLocation` _adscamera))
  (bind _returnvalue_2 (`SceneComponent.K2_GetComponentLocation` _firstpersoncamera))
  ;[1 1 1] 보고있는것 라인트레이스로 확인하기
  (if (`self.FirstPersonCamera?`)
    (bind _outhit (`KismetSystemLibrary.LineTraceSingle` _returnvalue_2 (+ _returnvalue_2 (* (`KismetMathLibrary.GetForwardVector` (`SceneComponent.K2_GetComponentRotation` _firstpersoncamera)) 300.0)) "TraceTypeQuery1"))
    (set `self.LookAtActor` (`.HitActor` (`GameplayStatics.BreakHitResult` _outhit)))
    (else
      (bind _outhit_2 (`KismetSystemLibrary.LineTraceSingle` _returnvalue (+ _returnvalue (* (`KismetMathLibrary.GetForwardVector` (`SceneComponent.K2_GetComponentRotation` _adscamera)) 450.0)) "TraceTypeQuery1"))
      (set `self.LookAtActor` (`.HitActor` (`GameplayStatics.BreakHitResult` _outhit_2))))))

(event `DropItem_Client`
  (params (Item :type "/Game/blueprints/Item/S_ItemDetails Structure"))
  (bind _inventory (`self.Inventory`))
  ;[1 1 1] 아이템 드롭
  (`KismetArrayLibrary.Array_Remove` _inventory (`KismetArrayLibrary.Array_Find` _inventory Item))
  (bind _output_get (set `self.DropItem` (== (`StaticMeshComponent.StaticMesh` (`self.UseItemMesh`)) (`.ItemMesh_23_1B190C32491D881F27A43195A8D8ACAC` (break `/Game/blueprints/Item/S_ItemDetails` Item)))))
  (if _output_get
    (`self.SetSlot_Client` (`self.DefaultItem`)))
  (`self.DropItem_Server` Item))

(event `DropItem_Server`
  (params (Item :type "/Game/blueprints/Item/S_ItemDetails Structure"))
  ;[1 1 1] 아이템 드롭
  (`|SpawnActorFromClass` (`.Class_24_2FB023464498AE897DC388865F9B1FBF` (break `/Game/blueprints/Item/S_ItemDetails` Item)) (`SceneComponent.K2_GetComponentToWorld` (`self.DropLocation`)) "AdjustIfPossibleButAlwaysSpawn" "OverrideRootScale" null null))

(event `SetSlot_Client`
  (params (Slot1 :type "/Game/blueprints/Item/S_ItemDetails Structure"))
  ;[1 1 1] 사용가능한 아이템 슬롯
  (`self.SetSlot_Server` Slot1))

(event `SetSlot_Server`
  (params (Slot1 :type "/Game/blueprints/Item/S_ItemDetails Structure"))
  ;[1 1 1] 사용가능한 아이템 슬롯
  (set `self.Slot1` Slot1) ; RepNotify로 된 변수들은 변경사항이 있으면 불러옴
)

(event `InputAction|CheatMode`
  (params (Key :type "Key Structure"))
  ;[1 1 1] 치트모드
  (:`Pressed`
    (set `CharacterMovementComponent.MaxWalkSpeed` 3000.0 (`self.CharacterMovement`))))

(fn `OnRep_Slot1`
  (bind _useitemmesh (`self.UseItemMesh`))
  (bind (_name _descripsion _thumbnail _itemmesh _class _student1_bs _student2_bs _socketname) (break `/Game/blueprints/Item/S_ItemDetails` (`self.Slot1`)))
  (bind _returnvalue (`SkeletalMeshComponent.GetAnimInstance` (`self.Mesh`)))
  ;[1 1 1] 클라이언트가 서버에 정보 받기도 전에 변수 실행되면 안되서 REPNOTICE로 함
  (`StaticMeshComponent.SetStaticMesh` _useitemmesh _itemmesh)
  (`SceneComponent.K2_AttachToComponent` _useitemmesh (`self.Mesh`) _socketname "SnapToTarget" "SnapToTarget" "SnapToTarget" false)
  (if (`self.Student1?`)
    (set `/Game/Animation/PNAnimBP_Student.EquipBS` _student1_bs (cast `/Game/Animation/PNAnimBP_Student` _returnvalue :!pure true))
    (else
      (set `/Game/Animation/PNAnimBP_Student2.EquipBS` _student2_bs (cast `/Game/Animation/PNAnimBP_Student2` _returnvalue :!pure true)))))

(fn `UserConstructionScript`)